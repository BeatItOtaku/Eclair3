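; ArchiveActor is a collectible archive pickup that records itself in the player's stage save.
; The first sphere overlap plays a Wwise sound, waits briefly, adds its ID to the current stage's obtained keys, saves, then destroys the actor.
; In the editor, the construction script fills an empty ID from the level name plus the count of ArchiveActors already having IDs.
; A mesh-rotation timeline exists but never runs.
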(event `self.ReceiveBeginPlay`
  (bind _aseclair_game_instance (cast `/Game/Base/Blueprint/EclairGameInstance` (`GameplayStatics.GetGameInstance`)))
  (set `self.GameInstance` _aseclair_game_instance))

(event `self.Sphere.OnComponentBeginOverlap`
  (params (OverlappedComponent :type "PrimitiveComponent Object Reference") (OtherActor :type "Actor Object Reference") (OtherComp :type "PrimitiveComponent Object Reference") (OtherBodyIndex :type Integer) (bFromSweep :type Boolean) (SweepResult :type "HitResult Structure (by ref)"))
  (bind (_currentstagestate_time _currentstagestate_obtaineditems _currentstagestate_obtainedkeys) (break `/Game/Base/Blueprint/SaveData/StageState` (`/Game/Base/Blueprint/EclairGameInstance.CurrentStageState` (`self.GameInstance`))))
  (`/Engine/EditorBlueprintResources/StandardMacros.DoOnce` false
    (:`Completed`
      (`AkGameplayStatics.PostEvent` "/Game/Sound/SE/System/GetArchive.GetArchive" self)
      (`KismetSystemLibrary.Delay` 0.27)
      (`|ExecutionSequence`
        (:`then_0`
          (`BlueprintSetLibrary.Set_Add` _currentstagestate_obtainedkeys (`self.ID`))
          (`/Game/Base/Blueprint/EclairGameInstance.SaveCurrentStage` (`self.GameInstance`)))
        (:`then_1`
          (`self.K2_DestroyActor`))))))

(event `self.Sphere.OnComponentEndOverlap`
  (params (OverlappedComponent :type "PrimitiveComponent Object Reference") (OtherActor :type "Actor Object Reference") (OtherComp :type "PrimitiveComponent Object Reference") (OtherBodyIndex :type Integer)))

(fn `UserConstructionScript`
  (locals (temp_actorcount :type Integer))
  ;[1 1 1] IDが無かったら付与
  (bind _returnvalue (`AkGameplayStatics.IsEditor`))
  (if _returnvalue
    (if (`KismetStringLibrary.EqualEqual_StrStr` (`self.ID`))
      (bind _outactors (`GameplayStatics.GetAllActorsOfClass` "ArchiveActor_C"))
      (for _array_element _outactors
        (if (`KismetStringLibrary.NotEqual_StrStr` (`/Game/Gimmick/Archive/Blueprints/ArchiveActor.ID` _array_element))
          (`/Engine/EditorBlueprintResources/StandardMacros.IncrementInt` (`local.temp_actorcount`))))
      (bind _returnvalue_2 (`GameplayStatics.GetCurrentLevelName` true))
      (set `self.ID` (`KismetTextLibrary.Conv_TextToString` (`|FormatText` "{LevelName}{ID}" (`KismetTextLibrary.Conv_StringToText` _returnvalue_2) (`local.temp_actorcount`)))))))