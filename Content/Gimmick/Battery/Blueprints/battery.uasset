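; Battery pickup that the Eclair character collects to raise its battery count.
; The actor sets a fixed starting rotation, then spins its static mesh in yaw every tick.
; When the mesh overlaps EclairBP, it increments BatteryCount, posts a Wwise notify sound on the player controller, shows the new count through HUD_UI and destroys itself.
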(event `self.ReceiveBeginPlay`
  (`self.K2_SetActorRotation` (struct :`Pitch` 45.0)))

(event `self.ReceiveTick`
  (params (DeltaSeconds :type "Float (single-precision)"))
  (`SceneComponent.K2_AddWorldRotation` (`self.StaticMesh`) (`KismetMathLibrary.MakeRotator` 0.0 0.0 3.0) false false))

(event `self.StaticMesh.OnComponentBeginOverlap`
  (params (OverlappedComponent :type "PrimitiveComponent Object Reference") (OtherActor :type "Actor Object Reference") (OtherComp :type "PrimitiveComponent Object Reference") (OtherBodyIndex :type Integer) (bFromSweep :type Boolean) (SweepResult :type "HitResult Structure (by ref)"))
  (bind _returnvalue (`GameplayStatics.GetPlayerController` 0))
  (bind _aseclair_bp (cast `/Game/Character/Eclair/Blueprints/EclairBP` OtherActor))
  (bind _output_get (set `/Game/Character/Eclair/Blueprints/EclairBP.BatteryCount` (+ (`/Game/Character/Eclair/Blueprints/EclairBP.BatteryCount` _aseclair_bp) 1) _aseclair_bp))
  (`AkGameplayStatics.PostEvent` "/Game/Sound/SE/System/Notify.Notify" _returnvalue)
  (bind _ashud_ui (cast `/Game/Base/Widget/HUD/HUD_UI` (`PlayerController.GetHUD` _returnvalue)))
  (`/Game/Base/Widget/HUD/HUD_UI.ShowBatteryCounter` _ashud_ui _output_get)
  (`self.K2_DestroyActor`))

(fn `UserConstructionScript`)