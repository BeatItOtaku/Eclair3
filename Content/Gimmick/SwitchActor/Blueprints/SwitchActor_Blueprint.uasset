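; Switch gimmick actor that Eclair toggles on or off, calling on/off events and swapping blue and red lights.
; A box collider, sized in the construction script, enables InteractableGimmickComponent registration while Eclair overlaps, waiting for its ground event if airborne.
; Interaction flips the state, applies negative damage to Eclair and starts a cooldown.
; A gated Tick times the cooldown, during which the switch is unusable.
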(event `self.Collider.OnComponentBeginOverlap`
  (params (OverlappedComponent :type "PrimitiveComponent Object Reference") (OtherActor :type "Actor Object Reference") (OtherComp :type "PrimitiveComponent Object Reference") (OtherBodyIndex :type Integer) (bFromSweep :type Boolean) (SweepResult :type "HitResult Structure (by ref)"))
  ;[1 1 1] エクレアがスイッチの使用範囲内に入った時
  (bind _aseclair_bp (cast `/Game/Character/Eclair/Blueprints/EclairBP` OtherActor))
  (set `self.Eclair` _aseclair_bp)
  (set `self.IsEclairInColliderBox` true)
  (if (`self.CanUseSwitch`)
    (if (`/Game/Character/Eclair/Blueprints/EclairBP.IsOnGround?` (`self.Eclair`))
      (`/Game/Base/Blueprint/Interactable/InteractableGimmickComponent.SetRegisteringEnabled` (`self.InteractableGimmickComponent`) true) ; エクレアがスイッチを切り替えられる状態にする
      (else
        (add `/Game/Character/Eclair/Blueprints/EclairBP.OnEclaironGround` (`self.Eclair`) (delegate `OnEclaironGround_イベント_0`))))))

(event `self.ReceiveBeginPlay`
  (`self.SetLightColor`) ; スイッチのライトの色、現在機能してない
)

(event `self.ReceiveTick`
  (params (DeltaSeconds :type "Float (single-precision)"))
  ;[1 1 1] スイッチが使用可能かどうか
  (`/Engine/EditorBlueprintResources/StandardMacros.Gate` true :!label _label
    (:`Exit`
      (bind _output_get (set `self.NotWorkingCurrentTime` (+ (`self.NotWorkingCurrentTime`) (`GameplayStatics.GetWorldDeltaSeconds`))))
      (if (>= _output_get (`self.NotWorkingTime`))
        (`self.WorkingTimeGate_Close`) ; EventTick内Gateを閉じる
      ))))

(event `OnEclaironGround_イベント_0`
  (`/Engine/EditorBlueprintResources/StandardMacros.DoOnce` false :!label _label_2
    (:`Completed`
      (`/Game/Base/Blueprint/Interactable/InteractableGimmickComponent.SetRegisteringEnabled` (`self.InteractableGimmickComponent`) true) ; エクレアがスイッチを切り替えられる状態にする
      (`/Game/Base/Blueprint/Interactable/InteractableGimmickComponent.OnActorBeginOverlap` (`self.InteractableGimmickComponent`) null (`self.Eclair`)))))

(event `WorkingTimeGate_Open`
  ;[1 1 1] スイッチが使用可能かどうか
  (set `self.CanUseSwitch` false) ; スイッチ側で操作を受け付けない
  (`/Game/Base/Blueprint/Interactable/InteractableGimmickComponent.SetRegisteringEnabled` (`self.InteractableGimmickComponent`) false) ; エクレアがスイッチを切り替えられない状態にする
  (goto _label :!via `Open`))

(event `self.Collider.OnComponentEndOverlap`
  (params (OverlappedComponent :type "PrimitiveComponent Object Reference") (OtherActor :type "Actor Object Reference") (OtherComp :type "PrimitiveComponent Object Reference") (OtherBodyIndex :type Integer))
  ;[1 1 1] エクレアがスイッチの使用範囲外に出た時
  (bind _aseclair_bp (cast `/Game/Character/Eclair/Blueprints/EclairBP` OtherActor))
  (set `self.Eclair` _aseclair_bp)
  (remove `/Game/Character/Eclair/Blueprints/EclairBP.OnEclaironGround` (`self.Eclair`) (delegate `OnEclaironGround_イベント_0`))
  (`|ExecutionSequence`
    (:`then_0`
      (goto _label_2 :!via `Reset`))
    (:`then_1`
      (set `self.IsEclairInColliderBox` false)
      (`/Game/Base/Blueprint/Interactable/InteractableGimmickComponent.SetRegisteringEnabled` (`self.InteractableGimmickComponent`) false) ; エクレアがスイッチを切り替えられない状態にする
    )))

(event `WorkingTimeGate_Close`
  ;[1 1 1] スイッチが使用可能かどうか
  (set `self.CanUseSwitch` true) ; スイッチ側で操作を受け付ける
  (set `self.NotWorkingCurrentTime` 0.0) ; 操作不可能時間のリセット
  (if (`self.IsEclairInColliderBox`)
    (`/Game/Base/Blueprint/Interactable/InteractableGimmickComponent.SetRegisteringEnabled` (`self.InteractableGimmickComponent`) false) ; エクレアがスイッチを切り替えられない状態にする
    (goto _label :!via `Close`)
    (else
      (goto _label :!via `Close`))))

(event `self.InteractableGimmickComponent.OnInteracted`
  (params (Sender :type "Actor Object Reference"))
  (`|ExecutionSequence`
    (:`then_0`
      (`self.WorkingTimeGate_Open`) ; スイッチが使えない時間を設定
      (bind _output_switchon (`self.Set/Get Switch On` false))
      (`self.Set/Get Switch On` (not _output_switchon) true))
    (:`then_1`
      (`GameplayStatics.ApplyDamage` (`self.Eclair`) -1.0))))

(fn `Set/Get Switch On`
  (params (Input_SwitchOn :type Boolean) (IsSetter :type Boolean))
  (returns (output_SwitchOn :type Boolean))
  (bind _redlight (`self.RedLight`))
  (bind _bluelight (`self.BlueLight`))
  (if IsSetter
    (bind _output_get (set `self.IsSwitchOn` Input_SwitchOn))
    (if _output_get
      (`self.On Switch On`)
      (`SceneComponent.SetVisibility` _bluelight true true)
      (`SceneComponent.SetVisibility` _redlight false true)
      (else
        (`self.On Switch Off`)
        (`SceneComponent.SetVisibility` _bluelight false true)
        (`SceneComponent.SetVisibility` _redlight true true)))
    (else
      (return (`self.IsSwitchOn`)))))

(fn `SetLightColor`
  (bind _redlight (`self.RedLight`))
  (bind _bluelight (`self.BlueLight`))
  (if (`self.IsSwitchOn`)
    (`SceneComponent.SetVisibility` _bluelight true true)
    (`SceneComponent.SetVisibility` _redlight false true)
    (else
      (`SceneComponent.SetVisibility` _bluelight false true)
      (`SceneComponent.SetVisibility` _redlight true true))))

(fn `SetNotWorkingCurrentTime`
  (set `self.NotWorkingCurrentTime` (`self.NotWorkingTime`)))

(fn `SetNotWorkingTime`
  (params (NotWorkingTime :type "Float (double-precision)"))
  (set `self.NotWorkingTime` NotWorkingTime))

(fn `UserConstructionScript`
  (`BoxComponent.SetBoxExtent` (`self.Collider`) (`self.BoxColliderScale`) true))