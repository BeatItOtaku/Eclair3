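; Naraku is a pit-style gimmick actor that sends the player character (EclairBP) back to a respawn point when it overlaps the actor.
; On overlap it fades out the HUD, disables input and, after a delay, moves the character to the checked RespawnPoint_Blueprint with the latest CheckedTime.
; It then fades back in, applies damage after another delay and restores input.
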(event `self.ReceiveBeginPlay`
  (bind _ashud_ui (cast `/Game/Base/Widget/HUD/HUD_UI` (`PlayerController.GetHUD` (`GameplayStatics.GetPlayerController` 0))))
  (set `self.HUD` _ashud_ui))

(event `self.ReceiveActorBeginOverlap`
  (params (OtherActor :type "Actor Object Reference"))
  (bind _aseclair_bp (cast `/Game/Character/Eclair/Blueprints/EclairBP` OtherActor))
  (`/Game/Base/Widget/HUD/HUD_UI.FadeOut` (`self.HUD`))
  (bind _output_get (set `self.Eclair` _aseclair_bp))
  (`self.DisableInput` (`self.Eclair`) null)
  (`KismetSystemLibrary.Delay` 1.0)
  (`|ExecutionSequence`
    (:`then_0`
      (bind _outactors (`GameplayStatics.GetAllActorsOfClass` "/Game/Gimmick/Naraku/Blueprints/RespawnPoint_Blueprint.RespawnPoint_Blueprint_C"))
      (bind _latest (`self.Get Latest RespawnPoint` _outactors)))
    (:`then_1`
      (`self.K2_SetActorLocation` (`self.Eclair`) (`self.K2_GetActorLocation` _latest) false false)
      (`SceneComponent.SetVisibility` (`Character.Mesh` (`self.Eclair`)) true false))
    (:`then_2`
      (`/Game/Base/Widget/HUD/HUD_UI.FadeIn` (`self.HUD`))
      (`KismetSystemLibrary.Delay` 1.0)
      (`GameplayStatics.ApplyDamage` (`self.Eclair`) 1.0)
      (`self.EnableInput` (`self.Eclair`) null))))

(fn `Get Latest RespawnPoint`
  (params (SpawnPoints :type "Array of /Game/Gimmick/Naraku/Blueprints/RespawnPoint_Blueprint Object Reference"))
  (returns (Latest :type "/Game/Gimmick/Naraku/Blueprints/RespawnPoint_Blueprint Object Reference"))
  (locals (mLatest :type "/Game/Gimmick/Naraku/Blueprints/RespawnPoint_Blueprint Object Reference") (mLatestTime :type "Float (double-precision)"))
  (for _array_element SpawnPoints
    (if (`/Game/Gimmick/Naraku/Blueprints/RespawnPoint_Blueprint.Checked` _array_element)
      (bind _checkedtime (`/Game/Gimmick/Naraku/Blueprints/RespawnPoint_Blueprint.CheckedTime` _array_element))
      (if (> _checkedtime (`local.mLatestTime`))
        (set `local.mLatest` _array_element)
        (set `local.mLatestTime` _checkedtime))))
  (return (`local.mLatest`)))

(fn `UserConstructionScript`)