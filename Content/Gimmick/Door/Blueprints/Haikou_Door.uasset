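; Haikou_Door is a gimmick double sliding door that opens and closes, optionally driven by a linked SwitchActor.
; Both switch on and off events toggle the door from its IsOpen state, ignored while DoorMoving is set.
; Its OnOpenning and OnClosing dispatchers play separate timelines that slide the two panels in mirrored X directions.
; The construction script places the panels at open or closed marker components to match IsOpen.
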(event `self.ReceiveBeginPlay`
  (bind _switchactor (`self.SwitchActor`))
  (`|ExecutionSequence`
    (:`then_0`
      ;[1 1 1] ドアが開く時
      (add `self.OnOpenning` (delegate `OnOpenning_Event`)))
    (:`then_1`
      ;[1 1 1] ドアが閉じる時
      (add `self.OnClosing` (delegate `OnClosing_Event`)))
    (:`then_2`
      ;[1 1 1] スイッチがある場合、ＯｎＯｆｆで動作を開け閉めを入れ替える
      (`/Engine/EditorBlueprintResources/StandardMacros.IsValid` (`self.SwitchActor`)
        (:`Is Valid`
          (add `/Game/Gimmick/Switch/Blueprints/SwitchActor_Blueprint.On Switch On` _switchactor (delegate `On Switch On_イベント_0`))
          (add `/Game/Gimmick/Switch/Blueprints/SwitchActor_Blueprint.On Switch Off` _switchactor (delegate `On Switch Off_イベント_0`)))))))

(event `OnOpenning_Event`
  ;[1 1 1] ドアが開く時
  (bind (_direction _doorposition) (`Timeline|Open_Timeline` :!via `PlayFromStart`)
    (:`Update`
      (`SceneComponent.K2_SetRelativeLocation` (`self.DoorRight`) (`KismetMathLibrary.MakeVector` _doorposition) false false)
      (`SceneComponent.K2_SetRelativeLocation` (`self.DoorLeft`) (`KismetMathLibrary.MakeVector` (* _doorposition -1.0)) false false))
    (:`Finished`
      (set `self.isOpen` true)
      (set `self.DoorMoving` false))))

(event `OnClosing_Event`
  ;[1 1 1] ドアが閉じる時
  (bind (_direction _doorposition) (`Timeline|タイムライン_0` :!via `PlayFromStart`)
    (:`Update`
      (`SceneComponent.K2_SetRelativeLocation` (`self.DoorRight`) (`KismetMathLibrary.MakeVector` _doorposition) false false)
      (`SceneComponent.K2_SetRelativeLocation` (`self.DoorLeft`) (`KismetMathLibrary.MakeVector` (* _doorposition -1.0)) false false))
    (:`Finished`
      (set `self.isOpen` false)
      (set `self.DoorMoving` false))))

(event `On Switch Off_イベント_0`
  ;[1 1 1] スイッチがある場合、ＯｎＯｆｆで動作を開け閉めを入れ替える
  (if (not (`self.DoorMoving`)) :!label _label
    (if (`self.isOpen`)
      (`self.OnClosing`)
      (else
        (`self.OnOpenning`)))
    (set `self.DoorMoving` true)))

(event `On Switch On_イベント_0`
  ;[1 1 1] スイッチがある場合、ＯｎＯｆｆで動作を開け閉めを入れ替える
  (goto _label))

(fn `UserConstructionScript`
  (bind _returnvalue (`SceneComponent.K2_GetComponentLocation` (`self.ClosingPosition`)))
  (if (`self.isOpen`)
    (`SceneComponent.K2_SetWorldLocation` (`self.DoorLeft`) (`SceneComponent.K2_GetComponentLocation` (`self.OpenningPositionL`)) false false)
    (`SceneComponent.K2_SetWorldLocation` (`self.DoorRight`) (`SceneComponent.K2_GetComponentLocation` (`self.OpenningPositionR`)) false false)
    (else
      (`SceneComponent.K2_SetWorldLocation` (`self.DoorLeft`) _returnvalue false false)
      (`SceneComponent.K2_SetWorldLocation` (`self.DoorRight`) _returnvalue false false))))