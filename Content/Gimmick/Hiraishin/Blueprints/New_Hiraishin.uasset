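; Lightning rod (Hiraishin) gimmick that jams the Eclair player's ETO inside a configurable sphere zone.
; BeginPlay sizes the zone and spawns a purple particle effect scaled to its radius.
; Overlap begin and end call EtoJammer, which sets the player's jammed flag, swing-by permission, jamming spot and rotated axis, turning Eclair toward the rod during ETO.
; An optional SwitchActor disables both effect spawning and jamming updates while on.
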(event `self.ReceiveBeginPlay`
  (`SphereComponent.SetSphereRadius` (`self.ParticleZone`) (`self.SphereRadius`) true)
  (`/Engine/EditorBlueprintResources/StandardMacros.IsValid` (`self.SwitchActor`)
    (:`Is Valid`
      (if (not (`/Game/Gimmick/Switch/Blueprints/SwitchActor_Blueprint.SwitchOn` (`self.SwitchActor`)))
        (bind _returnvalue (`GameplayStatics.SpawnEmitterAtLocation` "/Game/Effects/FX_LightningRod_purple.FX_LightningRod_purple" (`SceneComponent.K2_GetComponentLocation` (`self.ParticleZone`)) (struct) (* (`self.ParticleSize`) (/ (`self.SphereRadius`) 200.0)) false :!label _label))
        (set `self.Particle_Blue` _returnvalue)))
    (:`Is Not Valid`
      (goto _label))))

(event `self.ReceiveTick`
  (params (DeltaSeconds :type "Float (single-precision)")))

(event `self.ParticleZone.OnComponentBeginOverlap`
  (params (OverlappedComponent :type "PrimitiveComponent Object Reference") (OtherActor :type "Actor Object Reference") (OtherComp :type "PrimitiveComponent Object Reference") (OtherBodyIndex :type Integer) (bFromSweep :type Boolean) (SweepResult :type "HitResult Structure (by ref)"))
  (`self.EtoJammer` OtherActor (`self.CanSwingBy`) true))

(event `self.ParticleZone.OnComponentEndOverlap`
  (params (OverlappedComponent :type "PrimitiveComponent Object Reference") (OtherActor :type "Actor Object Reference") (OtherComp :type "PrimitiveComponent Object Reference") (OtherBodyIndex :type Integer))
  (`self.EtoJammer` OtherActor (`self.CanSwingBy`)))

(fn `EtoJammer`
  (params (Actor :type "Actor Object Reference") (`Swing-By` :type Boolean) (EtoJammaered :type Boolean))
  (locals (`CanSwing-By` :type Boolean))
  (bind _player (`self.Player`))
  (bind _player_2 (`self.Player`))
  (bind _player_3 (`self.Player`))
  (bind _returnvalue (`SceneComponent.K2_GetComponentLocation` (`Actor.RootComponent` _player_2)))
  (bind (_returnvalue_x _returnvalue_y) (`KismetMathLibrary.BreakVector` (`KismetMathLibrary.Normal` (- (`self.JammingSpot`) _returnvalue))))
  (`/Engine/EditorBlueprintResources/StandardMacros.IsValid` (`self.SwitchActor`)
    (:`Is Valid`
      (if (not (`/Game/Gimmick/Switch/Blueprints/SwitchActor_Blueprint.SwitchOn` (`self.SwitchActor`)))
        (set `local.CanSwing-By` `Swing-By` :!label _label)
        (bind _aseclair_bp (cast `/Game/Character/Eclair/Blueprints/EclairBP` Actor))
        (bind _output_get (set `self.Player` _aseclair_bp))
        (`/Game/Character/Eclair/Blueprints/EclairBP.Set/Get_CanSwing-By` _output_get (`self.CanSwingBy`) true)
        (set `/Game/Character/Eclair/Blueprints/EclairBP.ETOJammered` EtoJammaered (`self.Player`))
        (bind _output_get_2 (set `/Game/Character/Eclair/Blueprints/EclairBP.JammingSpot` (`SceneComponent.K2_GetComponentLocation` (`self.ParticleZone`)) _player_2))
        (bind _output_get_3 (set `self.JammingSpot` _output_get_2))
        (set `/Game/Character/Eclair/Blueprints/EclairBP.ETOPosition` (- _returnvalue _output_get_3) _player_3)
        (if (`/Game/Character/Eclair/Blueprints/EclairBP.PlayETO` _player_3)
          (`self.K2_SetActorRotation` (`self.Player`) (`KismetMathLibrary.FindLookAtRotation` (`SceneComponent.K2_GetComponentLocation` (`Actor.RootComponent` _player_3)) (`self.JammingSpot`)) false) ; エクレアを避雷針の中心に向けさせる
        )
        (set `/Game/Character/Eclair/Blueprints/EclairBP.HiraishinAxis` (`KismetMathLibrary.GreaterGreater_VectorRotator` (`KismetMathLibrary.MakeVector` _returnvalue_x _returnvalue_y) (struct :`Yaw` 90.0)) (`self.Player`))
        (`/Game/Character/Eclair/Blueprints/EclairBP.SetJammeredEtoPosition` _player _player (`self.JammingSpot`))))
    (:`Is Not Valid`
      (goto _label))))

(fn `UserConstructionScript`)