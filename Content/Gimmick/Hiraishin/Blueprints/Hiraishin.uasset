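; Lightning rod (Hiraishin) gimmick that jams Eclair's ETO state inside a spherical zone.
; BeginPlay sizes the zone and, unless a linked switch starts on, spawns a scaled purple effect and records the jamming center.
; Overlap during ETO play passes Eclair the center, relative position and rotated axis, turns Eclair toward the center, and shows an escape UI.
; Leaving reruns that update with jamming off and removes the UI.
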(event `self.ReceiveBeginPlay`
  ;[1 1 1] 避雷針エフェクトを避雷針の大きさに合わせて表示
  (`SphereComponent.SetSphereRadius` (`self.ParticleZone`) (`self.SphereRadius`) true)
  (`/Engine/EditorBlueprintResources/StandardMacros.IsValid` (`self.SwitchActor`)
    (:`Is Valid`
      (if (not (`/Game/Gimmick/SwitchActor/Blueprints/SwitchActor_Blueprint.IsSwitchOn` (`self.SwitchActor`)))
        (bind _returnvalue (`GameplayStatics.SpawnEmitterAtLocation` "/Game/Effects/FX_LightningRod_purple.FX_LightningRod_purple" (`SceneComponent.K2_GetComponentLocation` (`self.ParticleZone`)) (struct) (* (`self.ParticleSize`) (/ (`self.SphereRadius`) 200.0)) false :!label _label))
        (set `self.Particle_Blue` _returnvalue)
        (set `self.JammingSpot` (`SceneComponent.K2_GetComponentLocation` (`self.ParticleZone`))) ; 避雷針効果範囲の中心位置を設定
      ))
    (:`Is Not Valid`
      (goto _label))))

(event `self.ReceiveTick`
  (params (DeltaSeconds :type "Float (single-precision)")))

(event `self.ParticleZone.OnComponentBeginOverlap`
  (params (OverlappedComponent :type "PrimitiveComponent Object Reference") (OtherActor :type "Actor Object Reference") (OtherComp :type "PrimitiveComponent Object Reference") (OtherBodyIndex :type Integer) (bFromSweep :type Boolean) (SweepResult :type "HitResult Structure (by ref)"))
  (bind _aseclair_bp (cast `/Game/Character/Eclair/Blueprints/EclairBP` OtherActor))
  (bind _output_get (set `self.Eclair` _aseclair_bp))
  (if (`/Game/Character/Eclair/Blueprints/EclairBP.IsPlayETO` _output_get)
    (`self.EtoJammer` true)
    ;[1 1 1] 避雷針脱出用ＵＩ表示
    (`/Engine/EditorBlueprintResources/StandardMacros.IsValid` (`self.ExitUI`)
      (:`Is Not Valid`
        (bind _returnvalue (`|CreateWidget` "/Game/Base/Widget/ToolTip/ExitFromHiraishinUI.ExitFromHiraishinUI_C" (`GameplayStatics.GetPlayerController` 0)))
        (bind _output_get_2 (set `self.ExitUI` _returnvalue))
        (`UserWidget.AddToViewport` _output_get_2 0)))))

(event `self.ParticleZone.OnComponentEndOverlap`
  (params (OverlappedComponent :type "PrimitiveComponent Object Reference") (OtherActor :type "Actor Object Reference") (OtherComp :type "PrimitiveComponent Object Reference") (OtherBodyIndex :type Integer))
  (`self.EtoJammer` false)
  ;[1 1 1] 避雷針脱出用ＵＩ消去
  (`/Game/Base/Widget/ToolTip/ToolTip.Destroy` (`self.ExitUI`))
  (set `self.ExitUI` null))

(fn `EtoJammer`
  (params (EtoJammaered :type Boolean))
  (locals (EclairPosition :type "Vector Structure" :default (0.0 0.0 0.0)))
  (bind _eclair (`self.Eclair`))
  (bind (_returnvalue_x _returnvalue_y) (`KismetMathLibrary.BreakVector` (`KismetMathLibrary.Normal` (- (`self.JammingSpot`) (`local.EclairPosition`)))))
  (set `/Game/Character/Eclair/Blueprints/EclairBP.IsETOJammered` EtoJammaered (`self.Eclair`)) ; 避雷針効果範囲内に入ったかどうか
  (set `/Game/Character/Eclair/Blueprints/EclairBP.CenterOfHiraishin` (`self.JammingSpot`) _eclair) ; EclairBPに避雷針の中心位置の座標を渡す
  (set `local.EclairPosition` (`SceneComponent.K2_GetComponentLocation` (`Actor.RootComponent` _eclair))) ; 避雷針衝突時のEclairの位置
  (set `/Game/Character/Eclair/Blueprints/EclairBP.ETOPosInHiraishin` (- (`local.EclairPosition`) (`self.JammingSpot`)) (`self.Eclair`)) ; 避雷針の中心位置からEclairへの相対位置
  (`self.K2_SetActorRotation` (`self.Eclair`) (`KismetMathLibrary.FindLookAtRotation` (`SceneComponent.K2_GetComponentLocation` (`Actor.RootComponent` (`self.Eclair`))) (`self.JammingSpot`)) false) ; エクレアを避雷針の中心に向けさせる
  (set `/Game/Character/Eclair/Blueprints/EclairBP.HiraishinAxis` (`KismetMathLibrary.GreaterGreater_VectorRotator` (`KismetMathLibrary.MakeVector` _returnvalue_x _returnvalue_y) (struct :`Yaw` 90.0)) (`self.Eclair`)) ; 避雷針の軸を設定
)

(fn `UserConstructionScript`)