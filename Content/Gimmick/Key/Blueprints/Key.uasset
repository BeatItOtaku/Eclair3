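; Collectible key pickup that records itself in the stage save when overlapped.
; On first capsule overlap it plays a Wwise sound, adds its ID to the GameInstance's obtained keys, saves, and updates the HUD key count.
; After a short delay it fires OnObtained and destroys itself.
; In the editor, the construction script fills an empty ID from the level name plus the count of Keys with IDs.
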(event `self.ReceiveBeginPlay`
  (bind _aseclair_game_instance (cast `/Game/Base/Blueprint/EclairGameInstance` (`GameplayStatics.GetGameInstance`)))
  (set `self.GameInstance` _aseclair_game_instance))

(event `self.CapsuleCollision.OnComponentBeginOverlap`
  (params (OverlappedComponent :type "PrimitiveComponent Object Reference") (OtherActor :type "Actor Object Reference") (OtherComp :type "PrimitiveComponent Object Reference") (OtherBodyIndex :type Integer) (bFromSweep :type Boolean) (SweepResult :type "HitResult Structure (by ref)"))
  (bind (_currentstagestate_time _currentstagestate_obtaineditems _currentstagestate_obtainedkeys) (break `/Game/Base/Blueprint/SaveData/StageState` (`/Game/Base/Blueprint/EclairGameInstance.CurrentStageState` (`self.GameInstance`))))
  (`/Engine/EditorBlueprintResources/StandardMacros.DoOnce` false
    (:`Completed`
      (`AkGameplayStatics.PostEvent` "/Game/Sound/SE/System/GetKey.GetKey" self)
      (`KismetSystemLibrary.PrintString` (`KismetSystemLibrary.GetDisplayName` OtherActor))
      (`|ExecutionSequence`
        (:`then_0`
          (`BlueprintSetLibrary.Set_Add` _currentstagestate_obtainedkeys (`self.ID`))
          (`/Game/Base/Blueprint/EclairGameInstance.SaveCurrentStage` (`self.GameInstance`)))
        (:`then_1`
          ;[1 1 1] UIを表示
          (bind _ashud_ui (cast `/Game/Base/Widget/HUD/HUD_UI` (`PlayerController.GetHUD` (`GameplayStatics.GetPlayerController` 0))))
          (`/Game/Base/Widget/HUD/HUD_UI.SetKeyCount` _ashud_ui (`BlueprintSetLibrary.Set_Length` _currentstagestate_obtainedkeys)))
        (:`then_2`
          (`KismetSystemLibrary.Delay` 0.27)
          (`self.OnObtained`)
          (`self.K2_DestroyActor`))))))

(fn `UserConstructionScript`
  (locals (temp_actorcount :type Integer))
  ;[1 1 1] IDが無かったら付与
  (bind _returnvalue (`AkGameplayStatics.IsEditor`))
  (if _returnvalue
    (if (`KismetStringLibrary.EqualEqual_StrStr` (`self.ID`))
      (bind _outactors (`GameplayStatics.GetAllActorsOfClass` "Key_C"))
      (for _array_element _outactors
        (if (`KismetStringLibrary.NotEqual_StrStr` (`/Game/Gimmick/Key/Blueprints/Key.ID` _array_element))
          (`/Engine/EditorBlueprintResources/StandardMacros.IncrementInt` (`local.temp_actorcount`))))
      (bind _returnvalue_2 (`GameplayStatics.GetCurrentLevelName` true))
      (set `self.ID` (`KismetTextLibrary.Conv_TextToString` (`|FormatText` "{LevelName}{ID}" (`KismetTextLibrary.Conv_StringToText` _returnvalue_2) (`local.temp_actorcount`)))))))