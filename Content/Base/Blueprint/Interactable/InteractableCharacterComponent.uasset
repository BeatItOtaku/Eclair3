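; Character component that tracks the interactable gimmicks currently registered to it and picks which one to interact with.
; Register and unregister calls update the gimmick set, fire OnRegistered or OnUnregistered, and print the owner's name for debugging.
; GetInteractableGimmick scans the set and returns the highest-priority gimmick with a success flag, leaving the interaction itself to the caller.
; Terminate clears the set without firing OnUnregistered.
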(fn `GetInteractableGimmick`
  (returns (Suceed :type Boolean) (Gimmick :type "/Game/Base/Blueprint/Interactable/InteractableGimmickComponent Object Reference"))
  (locals (maxPriorityGimmick :type "/Game/Base/Blueprint/Interactable/InteractableGimmickComponent Object Reference"))
  (bind _maxprioritygimmick (`local.maxPriorityGimmick`))
  (bind _maxprioritygimmick_2 (`local.maxPriorityGimmick`))
  (set `local.maxPriorityGimmick` null)
  (bind _result (`BlueprintSetLibrary.Set_ToArray` (`self.InteractableGimmicks`)))
  ;[1 1 1] インタラクト可能なギミックの中でもっとも重要度が高いものを取得
  (for _array_element _result
    (`/Engine/EditorBlueprintResources/StandardMacros.IsValid` _maxprioritygimmick
      (:`Is Valid`
        (if (> (`/Game/Base/Blueprint/Interactable/InteractableGimmickComponent.Priority` _array_element) (`/Game/Base/Blueprint/Interactable/InteractableGimmickComponent.Priority` _maxprioritygimmick))
          (set `local.maxPriorityGimmick` _array_element :!label _label)))
      (:`Is Not Valid`
        (goto _label))))
  ;[1 1 1] インタラクトと後処理
  (`/Engine/EditorBlueprintResources/StandardMacros.IsValid` _maxprioritygimmick_2
    (:`Is Valid`
      (return true _maxprioritygimmick_2))
    (:`Is Not Valid`
      (return false null))))

(fn `RegisterInteractableGimmick`
  (params (Gimmick :type "/Game/Base/Blueprint/Interactable/InteractableGimmickComponent Object Reference"))
  (`BlueprintSetLibrary.Set_Add` (`self.InteractableGimmicks`) Gimmick)
  (`self.OnRegistered`)
  (`KismetSystemLibrary.PrintString` (`KismetSystemLibrary.GetObjectName` (`self.GetOwner` Gimmick))))

(fn `Terminate`
  (`BlueprintSetLibrary.Set_Clear` (`self.InteractableGimmicks`)))

(fn `UnregisterInteractableGimmick`
  (params (Gimmick :type "/Game/Base/Blueprint/Interactable/InteractableGimmickComponent Object Reference (by ref)"))
  (bind _returnvalue (`BlueprintSetLibrary.Set_Remove` (`self.InteractableGimmicks`) Gimmick))
  (if _returnvalue
    (`self.OnUnregistered`)
    (`KismetSystemLibrary.PrintString` (`KismetSystemLibrary.GetObjectName` (`self.GetOwner` Gimmick)) true true (struct :`R` 1.0 :`B` 0.098177 :`A` 1.0))))