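; Actor component that makes its owning gimmick actor interactable by characters that overlap it.
; Owner overlap events register and unregister it with the other actor's InteractableCharacterComponent, tracking those components in a collection.
; Registration on overlap can be switched off, which also unregisters it from every tracked character and clears the collection.
; Interact forwards the sender through the OnInteracted dispatcher.
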(event `self.ReceiveBeginPlay`
  (bind _returnvalue (`self.GetOwner`))
  (add `Actor.OnActorBeginOverlap` _returnvalue (delegate `OnActorBeginOverlap`))
  (add `Actor.OnActorEndOverlap` _returnvalue (delegate `OnActorEndOverlap`)))

(event `OnActorBeginOverlap`
  (params (OverlappedActor :type "Actor Object Reference") (OtherActor :type "Actor Object Reference"))
  (bind _returnvalue (`Actor.GetComponentByClass` OtherActor "/Game/Base/Blueprint/Interactable/InteractableCharacterComponent.InteractableCharacterComponent_C"))
  (if (`self.RegisteringEnabled`)
    (`/Game/Base/Blueprint/Interactable/InteractableCharacterComponent.RegisterInteractableGimmick` _returnvalue self)
    (`BlueprintSetLibrary.Set_Add` (`self.RegisteringCharacters`) _returnvalue)))

(event `OnActorEndOverlap`
  (params (OverlappedActor :type "Actor Object Reference") (OtherActor :type "Actor Object Reference"))
  (bind _returnvalue (`Actor.GetComponentByClass` OtherActor "/Game/Base/Blueprint/Interactable/InteractableCharacterComponent.InteractableCharacterComponent_C"))
  (`/Game/Base/Blueprint/Interactable/InteractableCharacterComponent.UnregisterInteractableGimmick` _returnvalue self)
  (`BlueprintSetLibrary.Set_Remove` (`self.RegisteringCharacters`) _returnvalue))

(event `Interact`
  (params (Sender :type "Actor Object Reference"))
  (`self.OnInteracted` Sender))

(fn `RegisteringEnabled?`
  (returns (RegisteringEnabled :type Boolean))
  (return (`self.RegisteringEnabled`)))

(fn `SetRegisteringEnabled`
  (params (RegisteringEnabled :type Boolean))
  (bind _registeringcharacters (`self.RegisteringCharacters`))
  (bind _output_get (set `self.RegisteringEnabled` RegisteringEnabled))
  (if (not _output_get)
    ;[1 1 1] すべてのキャラクターに対し登録解除
    (bind _result (`BlueprintSetLibrary.Set_ToArray` _registeringcharacters))
    (for _array_element _result
      (`/Game/Base/Blueprint/Interactable/InteractableCharacterComponent.UnregisterInteractableGimmick` _array_element self))
    (`BlueprintSetLibrary.Set_Clear` _registeringcharacters)))