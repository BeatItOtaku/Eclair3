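; Game mode for Chapter 1 that tracks play time, combat status and the result screen.
; Tick accumulates time while counting is enabled and writes it to the game instance; result requests show a widget with time and item totals.
; Enemies register as targeting entries, switching the isFighting state group between Fighting and None.
; Event dispatchers relay GUI focus, respawn, sequence skip, result close and targeted-enemy changes.
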(event `RequestResult`
  (params (Requestor :type "Actor Object Reference") (StageDefinition :type "StageDefinition Object Reference"))
  (bind (_currentstagestate_time _currentstagestate_obtaineditems) (break `/Game/Base/Blueprint/SaveData/StageState` (`/Game/Base/Blueprint/EclairGameInstance.CurrentStageState` (`self.GameInstance`))))
  ;[1 1 1] リザルト要求
  (bind _returnvalue (`|CreateWidget` "/Game/Base/Widget/Result/ResultUI.ResultUI_C" null (`KismetMathLibrary.FromSeconds` (`self.Time`)) (`BlueprintSetLibrary.Set_Length` _currentstagestate_obtaineditems) (`StageDefinition.ItemCount` StageDefinition) StageDefinition))
  (bind _output_get (set `self.ResultUI` _returnvalue))
  (`UserWidget.AddToViewport` _output_get 0))

(event `SetGUIFocus`
  (params (Location :type "Vector2D Structure"))
  ;[1 1 1] キー操作でGUIを選択してる時に出てくるカーソル
  (`self.OnGUIFocusSet` Location))

(event `CharacterRespawned`
  ;[1 1 1] リスポーン時処理
  (`self.OnCharacterRespawned`))

(event `DisableGUIFocus`
  ;[1 1 1] キー操作でGUIを選択してる時に出てくるカーソル
  (`self.OnGUIFocusDisabled`))

(event `SequenceSkipped`
  (`self.OnSequenceSkipped`))

(event `ResultClosed`
  ;[1 1 1] リザルト要求
  (`self.OnResultClosed`))

(event `self.ReceiveBeginPlay`
  (bind _aseclair_game_instance (cast `/Game/Base/Blueprint/EclairGameInstance` (`GameplayStatics.GetGameInstance`)))
  (set `self.GameInstance` _aseclair_game_instance)
  (set `self.Time` (`/Game/Base/Blueprint/EclairGameInstance.Time` _aseclair_game_instance)))

(event `self.ReceiveTick`
  (params (DeltaSeconds :type "Float (single-precision)"))
  ;[1 1 1] 経過時間のカウント
  (if (`self.TimeIsCounting`)
    (bind _output_get (set `self.Time` (+ DeltaSeconds (`self.Time`))))
    (set `/Game/Base/Blueprint/EclairGameInstance.Time` _output_get (`self.GameInstance`))))

(event `ResetTimeCounter`
  ;[1 1 1] 経過時間のカウント
  (set `self.Time` 0.0))

(fn `RegisterTargetedEnemies`
  (params (Enemy :type "Actor Object Reference"))
  (bind _targetedenemies (`self.TargetedEnemies`))
  (if (not (`BlueprintSetLibrary.Set_Contains` _targetedenemies Enemy))
    (`BlueprintSetLibrary.Set_Add` _targetedenemies Enemy)
    (`AkGameplayStatics.SetState` "isFighting" "Fighting")
    (`self.OnTargetedEnemiesChanged`)))

(fn `UnregisterTargetedEnemies`
  (params (Enemy :type "Actor Object Reference"))
  (bind _targetedenemies (`self.TargetedEnemies`))
  (bind _returnvalue (`BlueprintSetLibrary.Set_Remove` _targetedenemies Enemy))
  (if _returnvalue
    (`self.OnTargetedEnemiesChanged`)
    (if (== (`BlueprintSetLibrary.Set_Length` _targetedenemies) 0)
      (`AkGameplayStatics.SetState` "isFighting")
      (else
        (`AkGameplayStatics.SetState` "isFighting" "Fighting")))))

(fn `UserConstructionScript`)