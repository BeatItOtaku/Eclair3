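; Game instance for Eclair that owns the save game, current stage progress and session-wide settings.
; LoadData loads or creates the "Eclair" save slot, separately from Init, which defaults graphics to High via scalability console commands.
; OpenStage resets progress on stage change and clears audio states.
; Saving writes checkpoints, settings, or results merging collectibles and best times; it also tracks a widget stack and controller type, and relays Back input.
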(event `self.ReceiveInit`
  (`self.Set Graphic Quality` "NewEnumerator0"))

(event `LoadData`
  (bind _eclairsavegame (`self.EclairSaveGame`))
  (`|ExecutionSequence`
    (:`then_0`
      (bind _returnvalue (`GameplayStatics.LoadGameFromSlot` "Eclair"))
      (bind _aseclair_save_game (cast `/Game/Base/Blueprint/SaveData/EclairSaveGame` _returnvalue)
        (:`then`
          (set `self.EclairSaveGame` _aseclair_save_game))
        (:`CastFailed`
          (bind _returnvalue_2 (`GameplayStatics.CreateSaveGameObject` "/Game/Base/Blueprint/SaveData/EclairSaveGame.EclairSaveGame_C")) ; セーブデータがない(初回起動時)はセーブデータを作る
          (bind _output_get (set `self.EclairSaveGame` _returnvalue_2))
          (`GameplayStatics.SaveGameToSlot` _output_get "Eclair")
          (set `self.IsInitialLaunch` true))))
    (:`then_1`
      (bind _output_get_2 (set `self.CurrentStageState` (`/Game/Base/Blueprint/SaveData/EclairSaveGame.CurrentStageState` _eclairsavegame)))
      (set `self.Time` (`.Time_4_7999F8724670ABB3EF2A209583473F63` (break `/Game/Base/Blueprint/SaveData/StageState` _output_get_2)))
      (set `/Game/Base/Blueprint/SaveData/EclairSaveGame.Version` (`ResultEncryptor.GetProjectVersion`) _eclairsavegame)
      (`self.Set Graphic Quality` (`/Game/Base/Blueprint/SaveData/EclairSaveGame.GraphicQuality` _eclairsavegame)))))

(event `Press Back`
  ;[1 1 1] キーイベントをウィジェットで受け取るためのやつ
  (`self.InputEvent Press Back`))

(fn `Get Graphic Quality`
  (returns (GraphicQuality :type "/Game/Others/GraphicQuality Enum"))
  (return (`self.GraphicQuality`)))

(fn `GetControllerType`
  (returns (ControllerType :type "/Game/Base/Blueprint/ControllerType Enum"))
  (return (`self.ControllerType`)))

(fn `GetLastStageDefinition`
  (returns (StageDefinition :type "StageDefinition Object Reference"))
  (return (`self.StageDefinition`)))

(fn `Initialize`
  (set `self.CurrentStageState` (make `/Game/Base/Blueprint/SaveData/StageState` 0.0 (`|MakeSet`) (`|MakeSet`) (`|MakeSet`) (`|MakeSet`) (`|MakeMap`)))
  (set `self.ObtainedItems` (`|MakeSet`))
  (set `self.Time` 0.0))

(fn `IsInitialLaunch?`
  (returns (IsInitialLaunch :type Boolean))
  (return (`self.IsInitialLaunch`)))

(fn `OpenStage`
  (params (StageDefinition :type "StageDefinition Object Reference"))
  (`|ExecutionSequence`
    (:`then_0`
      (bind _output_get (set `self.StageDefinition` StageDefinition))
      (`GameplayStatics.OpenLevel` (`KismetStringLibrary.Conv_StringToName` (`StageDefinition.LevelName` _output_get)))
      (bind _slug (`StageDefinition.Slug` _output_get))
      ;[1 1 1] セーブデータと違うステージを開いたときは初期化
      (if (`KismetStringLibrary.NotEqual_StrStr` _slug (`/Game/Base/Blueprint/SaveData/EclairSaveGame.CurrentStage` (`self.EclairSaveGame`)))
        (set `/Game/Base/Blueprint/SaveData/EclairSaveGame.CurrentStage` _slug (`self.EclairSaveGame`))
        (`self.Initialize`)))
    (:`then_1`
      (`AkGameplayStatics.SetState` "Pausing")
      (`AkGameplayStatics.SetState` "BGMStates")
      (`AkGameplayStatics.SetState` "isFighting"))))

(fn `PopWidgetStack`
  (params (Widget :type "Object Object Reference"))
  (returns (Succeed :type Boolean))
  (bind _widgetstack (`self.WidgetStack`))
  (bind _returnvalue (`KismetArrayLibrary.Array_LastIndex` _widgetstack))
  (if (== (`|GetArrayItem` _widgetstack _returnvalue) Widget)
    (`KismetArrayLibrary.Array_Remove` _widgetstack _returnvalue)
    (return true)
    (else
      (return false))))

(fn `PushWidgetStack`
  (params (Widget :type "Widget Object Reference (by ref)"))
  (returns (Index :type Integer))
  (bind _returnvalue (`KismetArrayLibrary.Array_Add` (`self.WidgetStack`) Widget))
  (return _returnvalue))

(fn `SaveCurrentStage`
  (bind _eclairsavegame (`self.EclairSaveGame`))
  (bind (_currentstagestate_time _currentstagestate_obtaineditems _currentstagestate_obtainedkeys _currentstagestate_obtainedarchives _currentstagestate_playedconversations _currentstagestate_switchstates _currentstagestate_location) (break `/Game/Base/Blueprint/SaveData/StageState` (`self.CurrentStageState`)))
  (set `/Game/Base/Blueprint/SaveData/EclairSaveGame.CurrentStage` (`StageDefinition.Slug` (`self.StageDefinition`)) _eclairsavegame)
  (set `/Game/Base/Blueprint/SaveData/EclairSaveGame.CurrentStageState` (make `/Game/Base/Blueprint/SaveData/StageState` (`self.Time`) _currentstagestate_obtaineditems _currentstagestate_obtainedkeys _currentstagestate_obtainedarchives _currentstagestate_playedconversations _currentstagestate_switchstates _currentstagestate_location) _eclairsavegame)
  (`GameplayStatics.SaveGameToSlot` _eclairsavegame "Eclair")
  (set `self.continuesWhenRetry` true)
  (`self.OnSave`))

(fn `SaveResult`
  (params (StageDef :type "StageDefinition Object Reference"))
  (`self.SetResult` StageDef)
  (`GameplayStatics.SaveGameToSlot` (`self.EclairSaveGame`) "Eclair") ; セーブデータに書き込み
  (`self.OnSave`))

(fn `SaveSettings`
  (bind _eclairsavegame (`self.EclairSaveGame`))
  (set `/Game/Base/Blueprint/SaveData/EclairSaveGame.GraphicQuality` (`self.GraphicQuality`) _eclairsavegame)
  (`GameplayStatics.SaveGameToSlot` _eclairsavegame "Eclair")
  (`self.OnSave`))

(fn `Set Graphic Quality`
  (params (GraphicQuality :type "/Game/Others/GraphicQuality Enum" :default "NewEnumerator0"))
  (bind _output_get (set `self.GraphicQuality` GraphicQuality))
  (switch `/Game/Others/GraphicQuality` _output_get
    (:`NewEnumerator0`
      (`KismetSystemLibrary.ExecuteConsoleCommand` "sg.AntiAliasingQuality 2") ; アンチエイリアス
      (`KismetSystemLibrary.ExecuteConsoleCommand` "sg.PostProcessQuality 3") ; ポスプロ品質
      (`KismetSystemLibrary.ExecuteConsoleCommand` "sg.ShadowQuality 2") ; シャドウ品質
      (`KismetSystemLibrary.ExecuteConsoleCommand` "sg.TextureQuality 2") ; テクスチャ品質
      (`KismetSystemLibrary.ExecuteConsoleCommand` "r.ScreenPercentage 100") ; レンダリング解像度
      (`KismetSystemLibrary.ExecuteConsoleCommand` "sg.ViewDistanceQuality(2)") ; 描画距離
      (`KismetSystemLibrary.ExecuteConsoleCommand` "sg.EffectsQuality(2)") ; エフェクト品質
      (`KismetSystemLibrary.ExecuteConsoleCommand` "r.SSR.Quality 0") ; SSR
      (`KismetSystemLibrary.ExecuteConsoleCommand` "sg.FoliageQuality 3"))
    (:`NewEnumerator1`
      (`KismetSystemLibrary.ExecuteConsoleCommand` "sg.AntiAliasingQuality 0")
      (`KismetSystemLibrary.ExecuteConsoleCommand` "sg.PostProcessQuality 0")
      (`KismetSystemLibrary.ExecuteConsoleCommand` "sg.ShadowQuality 0")
      (`KismetSystemLibrary.ExecuteConsoleCommand` "sg.TextureQuality 0")
      (`KismetSystemLibrary.ExecuteConsoleCommand` "r.ScreenPercentage 100")
      (`KismetSystemLibrary.ExecuteConsoleCommand` "sg.ViewDistanceQuality(0)")
      (`KismetSystemLibrary.ExecuteConsoleCommand` "sg.EffectsQuality(0)")
      (`KismetSystemLibrary.ExecuteConsoleCommand` "r.SSR.Quality 0")
      (`KismetSystemLibrary.ExecuteConsoleCommand` "sg.FoliageQuality 1"))
    (:`NewEnumerator2`
      (`KismetSystemLibrary.ExecuteConsoleCommand` "sg.AntiAliasingQuality 0")
      (`KismetSystemLibrary.ExecuteConsoleCommand` "sg.PostProcessQuality 0")
      (`KismetSystemLibrary.ExecuteConsoleCommand` "sg.ShadowQuality 0")
      (`KismetSystemLibrary.ExecuteConsoleCommand` "sg.TextureQuality 0")
      (`KismetSystemLibrary.ExecuteConsoleCommand` "r.ScreenPercentage 50")
      (`KismetSystemLibrary.ExecuteConsoleCommand` "sg.ViewDistanceQuality(0)")
      (`KismetSystemLibrary.ExecuteConsoleCommand` "sg.EffectsQuality(0)")
      (`KismetSystemLibrary.ExecuteConsoleCommand` "r.SSR.Quality 0")
      (`KismetSystemLibrary.ExecuteConsoleCommand` "sg.FoliageQuality 0"))))

(fn `SetControllerType`
  (params (ControllerType :type "/Game/Base/Blueprint/ControllerType Enum" :default "NewEnumerator0"))
  (bind _output_get (set `self.ControllerType` ControllerType))
  (`self.OnControllerTypeChanged` _output_get))

(fn `SetResult`
  (params (StageDefinition :type "StageDefinition Object Reference"))
  (bind (_currentstagestate_time _currentstagestate_obtaineditems _currentstagestate_obtainedkeys _currentstagestate_obtainedarchives) (break `/Game/Base/Blueprint/SaveData/StageState` (`self.CurrentStageState`)))
  (bind _slug (`StageDefinition.Slug` StageDefinition))
  (bind _eclairsavegame (`self.EclairSaveGame`))
  (bind _value (`BlueprintMapLibrary.Map_Find` (`/Game/Base/Blueprint/SaveData/EclairSaveGame.StageResults` (`self.EclairSaveGame`)) _slug))
  (bind _result (`BlueprintSetLibrary.Set_Union` (`.ObtainedItems_13_4136E9F24A7F1636E2049FA709578893` (break `/Game/Base/Blueprint/SaveData/StageResult` _value)) _currentstagestate_obtaineditems)) ; 取ったデンチを合わせる
  (`BlueprintMapLibrary.Map_Add` (`/Game/Base/Blueprint/SaveData/EclairSaveGame.StageResults` _eclairsavegame) _slug (make `/Game/Base/Blueprint/SaveData/StageResult` (`KismetMathLibrary.SelectFloat` (`self.Time`) (break `/Game/Base/Blueprint/SaveData/StageResult` _value) (or (== 0.0 (break `/Game/Base/Blueprint/SaveData/StageResult` _value)) (> (break `/Game/Base/Blueprint/SaveData/StageResult` _value) (`self.Time`)))) _result))
  (bind _result_2 (`BlueprintSetLibrary.Set_Union` (`/Game/Base/Blueprint/SaveData/EclairSaveGame.ObtainedArchives` _eclairsavegame) _currentstagestate_obtainedarchives))
  (set `/Game/Base/Blueprint/SaveData/EclairSaveGame.ObtainedArchives` _result_2 _eclairsavegame))