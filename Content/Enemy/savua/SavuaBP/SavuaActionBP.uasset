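; Behavior tree task that runs a selected combat action for the Savua enemy, currently a three-hit sword attack.
; On execute it lazily caches the Savua AI controller, character and anim Blueprint, then switches on the action enum.
; The sword attack triggers the anim Blueprint and sets a fixed delay, after which the task finishes successfully rather than waiting on the animation.
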(event `self.ReceiveExecuteAI`
  (params (OwnerController :type "AIController Object Reference") (ControlledPawn :type "Pawn Object Reference"))
  (`self.SetAiCon&AiChara&AnimBP` OwnerController ControlledPawn)
  (switch `/Game/Enemy/savua/SavuaBP/SavuaActions` (`self.SavuaActions`)
    (:`NewEnumerator2`
      (`self.SwordAttack`)
      (`KismetSystemLibrary.Delay` (`self.DelayTime`))
      (`self.FinishExecute` true))))

(fn `SetAiCon&AiChara&AnimBP`
  (params (AiCon :type "Object Object Reference") (AiChara :type "Object Object Reference"))
  (`|ExecutionSequence`
    (:`then_0`
      (if (not (!= (`self.Savua_AiController`) null))
        (bind _assavua_ai_controller (cast `/Game/Enemy/savua/SavuaBP/Savua_AiController` AiCon))
        (set `self.Savua_AiController` _assavua_ai_controller)))
    (:`then_1`
      (if (not (!= (`self.Savua_AiCharacter`) null))
        (bind _assavua_ai_character (cast `/Game/Enemy/savua/SavuaBP/Savua_AiCharacter` AiChara))
        (set `self.Savua_AiCharacter` _assavua_ai_character))
      (if (not (!= (`self.Savua_AnimBP`) null))
        (bind _assavua_anim_bp (cast `/Game/Enemy/savua/SavuaAnim/SavuaAnimBP` (`SkeletalMeshComponent.GetAnimInstance` (`Character.Mesh` (`self.Savua_AiCharacter`)))))
        (set `self.Savua_AnimBP` _assavua_anim_bp)))))

(fn `SwordAttack`
  (`/Game/Enemy/savua/SavuaAnim/SavuaAnimBP.OnSwordAttack` (`self.Savua_AnimBP`)) ; 3連攻撃のモーション開始
  (set `self.DelayTime` 2.8))