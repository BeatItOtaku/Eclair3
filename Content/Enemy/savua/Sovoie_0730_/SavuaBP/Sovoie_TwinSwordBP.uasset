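; Twin sword Blueprint for the Sovoie enemy, playing an ice-themed sword formation (kensei) effect.
; The construction script puts a dynamic material instance on the TwinSword component.
; OnKensei_TwinSword runs a timeline that drives that material's ice_move parameter, then spawns scaled-up completion particles at two marker positions when it finishes.
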(event `OnKensei_TwinSword`
  (bind (_direction _ice_move) (`Timeline|タイムライン_0` :!via `PlayFromStart`)
    (:`Update`
      (`MaterialInstanceDynamic.SetScalarParameterValue` (`self.DMI_TwinSword`) "ice_move" _ice_move))
    (:`Finished`
      (`GameplayStatics.SpawnEmitterAtLocation` "/Game/Effects/FX_savua_kensei.FX_savua_kensei" (`SceneComponent.K2_GetComponentLocation` (`self.KenseiPosition1`)) (struct) (5.0 5.0 5.0)) ; 剣成後パーティクル表示
      (`GameplayStatics.SpawnEmitterAtLocation` "/Game/Effects/FX_savua_kensei.FX_savua_kensei" (`SceneComponent.K2_GetComponentLocation` (`self.KenseiPosition2`)) (struct) (5.0 5.0 5.0)) ; 剣成後パーティクル表示
    )))

(fn `UserConstructionScript`
  (bind _returnvalue (`PrimitiveComponent.CreateDynamicMaterialInstance` (`self.TwinSword`) 0 "/Game/Enemy/savua/Sovoie_0730_/katana/FXmat_savua_toushin_Inst.FXmat_savua_toushin_Inst"))
  (set `self.DMI_TwinSword` _returnvalue))