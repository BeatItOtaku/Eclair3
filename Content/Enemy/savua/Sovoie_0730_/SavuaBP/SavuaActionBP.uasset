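; Behavior tree task that executes one combat action for the Savua enemy, selected by an action enum.
; Per-action macros trigger animations and timed delays around drawing or breaking swords, melee attacks, guarding, damage reactions, and spawned ice shard fans or thrown twin swords.
; Helpers face and teleport relative to the blackboard target, Eclair.
; Some actions adjust a clamped attack stack, written to the blackboard before the task finishes.
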(event `self.ReceiveExecuteAI`
  (params (OwnerController :type "AIController Object Reference") (ControlledPawn :type "Pawn Object Reference"))
  (`self.SetAiCon&AiChara&AnimBP` OwnerController ControlledPawn)
  (switch `/Game/Enemy/savua/Sovoie_0730_/SavuaBP/SavuaActions` (`self.SavuaActions`)
    (:`NewEnumerator0`
      (`self.Idle_`
        (:`NewParam`
          _)))
    (:`NewEnumerator2`
      (`self.SwordAttack_`
        (:`NewParam`
          _)))
    (:`NewEnumerator3`
      (`self.TwinSwordAttack_`
        (:`NewParam`
          _)))
    (:`NewEnumerator4`
      (`self.ThrowTwinSword_`
        (:`NewParam`
          _)))
    (:`NewEnumerator5`
      (`self.IceShard_`
        (:`NewParam`
          _)))
    (:`NewEnumerator6`
      (`self.DrawSword_`
        (:`NewParam`
          _)))
    (:`NewEnumerator7`
      (`self.DrawTwinSword_`
        (:`NewParam`
          _)))
    (:`NewEnumerator12`
      (`self.Broken_` :!label _label
        (:`NewParam`
          _)))
    (:`NewEnumerator11`
      (goto _label :!via `FromGurad`))
    (:`NewEnumerator8`
      (`self.Guard_`
        (:`NewParam`
          _)))
    (:`NewEnumerator9`
      (`self.Damage_`))
    (:`NewEnumerator14`
      (`self.Teleportation` "NewEnumerator2")
      (`KismetSystemLibrary.Delay` (stale _delaytime) :!label _label_2))
    (:`NewEnumerator13`
      (`self.Teleportation` "NewEnumerator0")
      (goto _label_2))
    (:`NewEnumerator15`
      (bind _delaytime (`self.Teleportation` "NewEnumerator1"))
      (goto _label_2)))
  (`self.ResetVariables`)
  (`self.FinishExecute` true))

(fn `KnockBack`
  (locals (KnockBackScale :type "Float (double-precision)" :default 300.0))
  (bind (_returnvalue_x _returnvalue_y) (`KismetMathLibrary.BreakVector` (* (`KismetMathLibrary.Normal` (- (`Actor.K2_GetActorLocation` (`self.Savua_AiCharacter`)) (`BTFunctionLibrary.GetBlackboardValueAsVector` (`self.TargetLocation`)))) (`local.KnockBackScale`))))
  (`Actor.K2_AddActorWorldOffset` (`self.Savua_AiCharacter`) (`KismetMathLibrary.MakeVector` _returnvalue_x _returnvalue_y) true false))

(fn `LookAtEclair`
  (bind (_returnvalue_roll _returnvalue_pitch _returnvalue_yaw) (`KismetMathLibrary.BreakRotator` (`KismetMathLibrary.FindLookAtRotation` (`SceneComponent.K2_GetComponentLocation` (`Actor.RootComponent` (`self.Savua_AiCharacter`))) (`BTFunctionLibrary.GetBlackboardValueAsVector` (`self.TargetLocation`)))))
  (`SceneComponent.K2_SetWorldRotation` (`Actor.RootComponent` (`self.Savua_AiCharacter`)) (`KismetMathLibrary.MakeRotator` 0.0 0.0 _returnvalue_yaw) false false))

(fn `ResetVariables`
  (`BTFunctionLibrary.SetBlackboardValueAsBool` (`self.IsHitFromEclair`))
  (`BTFunctionLibrary.SetBlackboardValueAsInt` (`self.AttackStack`) (`self.AttackStackCount`)))

(fn `SetAiCon&AiChara&AnimBP`
  (params (AiCon :type "Object Object Reference") (AiChara :type "Object Object Reference"))
  (`|ExecutionSequence`
    (:`then_0`
      (if (not (!= (`self.Savua_AiController`) null))
        (bind _assavua_ai_controller (cast `/Game/Enemy/savua/Sovoie_0730_/SavuaBP/Savua_AiController` AiCon))
        (set `self.Savua_AiController` _assavua_ai_controller)))
    (:`then_1`
      (if (not (!= (`self.Savua_AiCharacter`) null))
        (bind _assavua_ai_character (cast `/Game/Enemy/savua/Sovoie_0730_/SavuaBP/Savua_AiCharacter` AiChara))
        (set `self.Savua_AiCharacter` _assavua_ai_character))
      (if (not (!= null null))
        (bind _assovoie_anim_bp (cast `/Game/Enemy/savua/Sovoie_0730_/SovoieAnimBP0730/SovoieAnimBP` (`SkeletalMeshComponent.GetAnimInstance` (`Character.Mesh` (`self.Savua_AiCharacter`)))))
        (set `self.Sovoie_AnimBP` _assovoie_anim_bp)))))

(fn `SetAttackStackCount`
  (params (AddStack :type Integer))
  (bind _output_get (set `self.AttackStackCount` (`KismetMathLibrary.Clamp` (+ (`self.AttackStackCount`) AddStack) 0 (`self.AttackStackMaxCount`))))
  (set `self.IsAttackStackMaxCount` (>= _output_get (`self.AttackStackMaxCount`))))

(fn `SettingIceShards`
  (locals (Angle :type "Float (double-precision)" :default -20.0))
  (`self.LookAtEclair`)
  (for _index (range 5)
    (`self.SpawnIceShard` (+ (`KismetMathLibrary.Conv_IntToDouble` (* _index 10)) (`local.Angle`)))))

(fn `SettingThorwingTwinSword`
  (bind _iceshardposition (`/Game/Enemy/savua/Sovoie_0730_/SavuaBP/Savua_AiCharacter.IceShardPosition` (`self.Savua_AiCharacter`)))
  (`self.LookAtEclair`)
  (`|SpawnActorFromClass` "/Game/Enemy/savua/Sovoie_0730_/SavuaBP/ThrowingTwinSword.ThrowingTwinSword_C" (`KismetMathLibrary.MakeTransform` (`SceneComponent.K2_GetComponentLocation` _iceshardposition) (`SceneComponent.K2_GetComponentRotation` _iceshardposition) (20.0 20.0 20.0)) "Undefined" "OverrideRootScale" null null)
  (`SceneComponent.SetVisibility` (`/Game/Enemy/savua/Sovoie_0730_/SavuaBP/Savua_AiCharacter.TwinSword` (`self.Savua_AiCharacter`)) false false) ; 両剣を非表示
  (`/Game/Enemy/savua/Sovoie_0730_/SavuaBP/Savua_AiController.OnSetNextDrawWeapon` (`self.Savua_AiController`)) ; 両剣を投げたため次に剣成する武器を選択する
)

(fn `SpawnIceShard`
  (params (Angle :type "Float (double-precision)"))
  (bind _iceshardposition (`/Game/Enemy/savua/Sovoie_0730_/SavuaBP/Savua_AiCharacter.IceShardPosition` (`self.Savua_AiCharacter`)))
  (bind (_returnvalue_roll _returnvalue_pitch _returnvalue_yaw) (`KismetMathLibrary.BreakRotator` (`SceneComponent.K2_GetComponentRotation` _iceshardposition)))
  (`|SpawnActorFromClass` "/Game/Enemy/savua/Sovoie_0730_/SavuaBP/IceShard.IceShard_C" (`KismetMathLibrary.MakeTransform` (`SceneComponent.K2_GetComponentLocation` _iceshardposition) (`KismetMathLibrary.MakeRotator` _returnvalue_roll _returnvalue_pitch (+ Angle _returnvalue_yaw))) "Undefined" "OverrideRootScale" null null))

(fn `Teleportation`
  (params (TeleportDirection :type "/Game/Enemy/savua/Sovoie_0730_/SavuaBP/TeleportationDirection Enum" :default "NewEnumerator0"))
  (returns (DelayTime :type "Float (double-precision)"))
  (locals (ScaleOfTeleport :type "Float (double-precision)" :default 100.0) (Direction :type "Vector Structure"))
  (bind _savua_aicharacter (`self.Savua_AiCharacter`))
  (bind (_returnvalue_x _returnvalue_y) (`KismetMathLibrary.BreakVector` (* (`local.Direction`) (`local.ScaleOfTeleport`))))
  (bind (_returnvalue_roll _returnvalue_pitch _returnvalue_yaw) (`KismetMathLibrary.BreakRotator` (`KismetMathLibrary.FindLookAtRotation` (`Actor.K2_GetActorLocation` _savua_aicharacter) (`BTFunctionLibrary.GetBlackboardValueAsVector` (`self.TargetLocation`)))))
  (bind _returnvalue (`KismetMathLibrary.Normal` (- (`Actor.K2_GetActorLocation` (`self.Savua_AiCharacter`)) (`BTFunctionLibrary.GetBlackboardValueAsVector` (`self.TargetLocation`)))))
  (switch `/Game/Enemy/savua/Sovoie_0730_/SavuaBP/TeleportationDirection` TeleportDirection
    (:`NewEnumerator0`
      (set `local.Direction` (* _returnvalue -1.0))
      (set `local.ScaleOfTeleport` 1500.0))
    (:`NewEnumerator1`
      (set `local.Direction` _returnvalue)
      (set `local.ScaleOfTeleport` 1500.0))
    (:`NewEnumerator2`
      (set `local.Direction` (`KismetMathLibrary.GreaterGreater_VectorRotator` (`KismetMathLibrary.MakeVector` (.x _returnvalue) (.y _returnvalue)) (`KismetMathLibrary.SelectRotator` (struct :`Yaw` 90.0) (struct :`Yaw` -90.0) (`KismetMathLibrary.Conv_IntToBool` (`KismetMathLibrary.RandomIntegerInRange` 0 1)))))
      (set `local.ScaleOfTeleport` 1000.0)))
  (`Actor.K2_AddActorWorldOffset` (`self.Savua_AiCharacter`) (`KismetMathLibrary.MakeVector` _returnvalue_x _returnvalue_y) true false)
  (`Actor.K2_SetActorRotation` _savua_aicharacter (`KismetMathLibrary.MakeRotator` 0.0 0.0 _returnvalue_yaw) false)
  (`/Game/Enemy/savua/Sovoie_0730_/SovoieAnimBP0730/SovoieAnimBP.OnBlink` (`self.Sovoie_AnimBP`))
  (return 1.4))