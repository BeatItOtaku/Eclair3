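; Savua enemy Blueprint, which equips itself with a katana when play begins.
; BeginPlay spawns a Katana_0626 actor, stores it, and attaches its root to the skeletal mesh's SwordSocket using KeepWorld rules.
; It then moves the katana to the socket's world location without explicitly setting rotation.
; Tick and overlap events are disabled, the construction script is empty, and some socket offset math is left unused.
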(event `self.ReceiveBeginPlay`
  (bind _returnvalue (`SceneComponent.GetSocketTransform` (`self.SkeletalMesh`) (`self.SwordSocket`) "RTS_World"))
  (bind _returnvalue_2 (`|SpawnActorFromClass` "/Game/Enemy/savua/katana_0626.katana_0626_C" (`self.SpawnTransform`) "Undefined" "OverrideRootScale" null null))
  (set `self.Katana` _returnvalue_2)
  (`SceneComponent.K2_AttachToComponent` (`Actor.RootComponent` (`self.Katana`)) (`self.SkeletalMesh`) (`self.SwordSocket`) "KeepWorld" "KeepWorld" "KeepWorld" true)
  (`SceneComponent.K2_SetWorldLocation` (`Actor.RootComponent` (`self.Katana`)) (`KismetMathLibrary.MakeVector` (.x (.location _returnvalue)) (.y (.location _returnvalue)) (.z (.location _returnvalue))) false false))

(fn `UserConstructionScript`)