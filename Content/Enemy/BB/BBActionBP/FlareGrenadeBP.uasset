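; Flare grenade projectile Blueprint for the BB enemy that damages the Eclair player character on contact.
; On BeginPlay it aims the grenade component once at the player's position, except in the VS_BB level.
; Tick then moves it along its forward vector by Speed per frame, without sweep or delta-time scaling.
; Any overlap spawns an explosion effect and destroys the grenade component, leaving the actor itself; only EclairBP takes damage.
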(event `self.ReceiveBeginPlay`
  (bind _returnvalue (`GameplayStatics.GetCurrentLevelName` true))
  (if (not (`KismetStringLibrary.EqualEqual_StrStr` _returnvalue "VS_BB"))
    (bind _aseclair_bp (cast `/Game/Character/Eclair/Blueprints/EclairBP` (`GameplayStatics.GetPlayerCharacter` 0)))
    (`SceneComponent.K2_SetWorldRotation` (`self.FlareGrenade`) (`KismetMathLibrary.FindLookAtRotation` (`SceneComponent.K2_GetComponentLocation` (`self.FlareGrenade`)) (`SceneComponent.K2_GetComponentLocation` (`Actor.RootComponent` _aseclair_bp))) false false)))

(event `self.ReceiveTick`
  (params (DeltaSeconds :type "Float (single-precision)"))
  (bind _flaregrenade (`self.FlareGrenade`))
  (`/Engine/EditorBlueprintResources/StandardMacros.IsValid` _flaregrenade
    (:`Is Valid`
      (`SceneComponent.K2_AddWorldOffset` (`self.FlareGrenade`) (* (`SceneComponent.GetForwardVector` _flaregrenade) (`self.speed`)) false false))))

(event `self.FlareGrenade.OnComponentBeginOverlap`
  (params (OverlappedComponent :type "PrimitiveComponent Object Reference") (OtherActor :type "Actor Object Reference") (OtherComp :type "PrimitiveComponent Object Reference") (OtherBodyIndex :type Integer) (bFromSweep :type Boolean) (SweepResult :type "HitResult Structure (by ref)"))
  (bind _aseclair_bp (cast `/Game/Character/Eclair/Blueprints/EclairBP` OtherActor)
    (:`then`
      (`GameplayStatics.ApplyDamage` _aseclair_bp 1.0 null self))
    (:`CastFailed`
      _))
  (`GameplayStatics.SpawnEmitterAtLocation` "/Game/Effects/FX_FlareGrenade_explode.FX_FlareGrenade_explode" (`SceneComponent.K2_GetComponentLocation` (`self.FlareGrenade`)))
  (`ActorComponent.K2_DestroyComponent` (`self.FlareGrenade`)))

(fn `UserConstructionScript`)