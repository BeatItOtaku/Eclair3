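; Construction-script Blueprint that builds a straight run of a repeated mesh capped by an end mesh.
; LoopMesh is instanced LoopCount times along the chosen X, Y or Z axis, spaced by its full bounds size plus LoopOffset.
; A second instanced component places EndMesh beyond the last copy, using its own bounds, LoopOffset and EndMeshOffset.
; The event graph holds only empty placeholder events.
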(fn `UserConstructionScript`
  (bind _loopmesh (`self.LoopMesh`))
  (bind _endmesh (`self.EndMesh`))
  (`|ExecutionSequence`
    (:`then_0`
      ;[1 1 1] Copy Offsetを計算
      (`StaticMeshComponent.SetStaticMesh` (`self.LoopInstancedStaticMesh`) _loopmesh)
      (switch `ESplineMeshAxis` (`self.LoopAxis`)
        (:`X`
          (set `self.AxisMask` (1.0 0.0 0.0)))
        (:`Y`
          (set `self.AxisMask` (0.0 1.0 0.0)))
        (:`Z`
          (set `self.AxisMask` (0.0 0.0 1.0))))
      (set `self.CopyOffset` (* (+ (* (`.BoxExtent` (`KismetMathLibrary.BreakBoxSphereBounds` (`StaticMesh.GetBounds` _loopmesh))) 2) (`self.LoopOffset`)) (`self.AxisMask`))))
    (:`then_1`
      ;[1 1 1] ループ部分を作成
      (for _index (range (`self.LoopCount`))
        (`InstancedStaticMeshComponent.AddInstance` (`self.LoopInstancedStaticMesh`) (`KismetMathLibrary.MakeTransform` (* (`self.CopyOffset`) _index)))))
    (:`then_2`
      ;[1 1 1] エンド部分を作成
      (`StaticMeshComponent.SetStaticMesh` (`self.EndInstancedStaticMesh`) _endmesh)
      (`InstancedStaticMeshComponent.AddInstance` (`self.EndInstancedStaticMesh`) (`KismetMathLibrary.MakeTransform` (+ (* (+ (* (`.BoxExtent` (`KismetMathLibrary.BreakBoxSphereBounds` (`StaticMesh.GetBounds` _endmesh))) 2) (`self.LoopOffset`)) (`self.AxisMask`)) (* (`self.CopyOffset`) (- (`self.LoopCount`) 1)) (`self.EndMeshOffset`)))))))