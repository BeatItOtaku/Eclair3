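; Lightning rod (hiraishin) actor that jams the player's ETO ability inside a spherical zone, passing along whether swing-by is allowed.
; BeginPlay sizes the zone and spawns a blue or red emitter by that flag; Tick removes the red one once a linked switch is on.
; Overlaps feed EtoJammer, which, unless that switch is on, sets the player's jam state, spot and perpendicular axis, turning the player toward the rod during ETO.
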(event `self.ReceiveBeginPlay`
  (bind _returnvalue (`SceneComponent.K2_GetComponentLocation` (`self.ParticleZone`)))
  (`SphereComponent.SetSphereRadius` (`self.ParticleZone`) (`self.SphereRadius`) true)
  (`/Engine/EditorBlueprintResources/StandardMacros.IsValid` (`self.SwitchActor`)
    (:`Is Valid`
      (if (not (`self.SwitchOn`))
        (if (`self.CanSwingBy`) :!label _label
          (bind _returnvalue_2 (`GameplayStatics.SpawnEmitterAtLocation` null _returnvalue (struct) (1.0 1.0 1.0) false))
          (set `self.Particle_Blue` _returnvalue_2)
          (else
            (bind _returnvalue_3 (`GameplayStatics.SpawnEmitterAtLocation` null _returnvalue (struct) (1.0 1.0 1.0) false))
            (set `self.Particle_Red` _returnvalue_3)))))
    (:`Is Not Valid`
      (goto _label))))

(event `self.ReceiveTick`
  (params (DeltaSeconds :type "Float (single-precision)"))
  (bind (_switchactor _switchactor_2) (`self.SwitchActor`))
  (`/Engine/EditorBlueprintResources/StandardMacros.IsValid` _switchactor
    (:`Is Valid`
      (if (`/Game/Import/Blueprints/New_Hiraishin.SwitchOn` _switchactor_2)
        (`/Engine/EditorBlueprintResources/StandardMacros.IsValid` (`self.Particle_Red`)
          (:`Is Valid`
            (`ActorComponent.K2_DestroyComponent` (`self.Particle_Red`))))))))

(event `self.ParticleZone.OnComponentBeginOverlap`
  (params (OverlappedComponent :type "PrimitiveComponent Object Reference") (OtherActor :type "Actor Object Reference") (OtherComp :type "PrimitiveComponent Object Reference") (OtherBodyIndex :type Integer) (bFromSweep :type Boolean) (SweepResult :type "HitResult Structure (by ref)"))
  (`self.EtoJammer` OtherActor (`self.CanSwingBy`) true))

(event `self.ParticleZone.OnComponentEndOverlap`
  (params (OverlappedComponent :type "PrimitiveComponent Object Reference") (OtherActor :type "Actor Object Reference") (OtherComp :type "PrimitiveComponent Object Reference") (OtherBodyIndex :type Integer))
  (`self.EtoJammer` OtherActor (`self.CanSwingBy`)))

(fn `EtoJammer`
  (params (Actor :type "Actor Object Reference") (`Swing-By` :type Boolean) (EtoJammaered :type Boolean))
  (locals (`CanSwing-By` :type Boolean))
  (bind (_player _player_2) (`self.Player`))
  (bind (_player_3 _player_4) (`self.Player`))
  (bind _returnvalue (`SceneComponent.K2_GetComponentLocation` (`Actor.RootComponent` _player_2)))
  (bind (_returnvalue_x _returnvalue_y) (`KismetMathLibrary.BreakVector` (`KismetMathLibrary.Normal` (- (`self.JammingSpot`) _returnvalue))))
  (`/Engine/EditorBlueprintResources/StandardMacros.IsValid` (`self.SwitchActor`)
    (:`Is Valid`
      (if (not (`/Game/Import/Blueprints/New_Hiraishin.SwitchOn` (`.SwitchActor` (`self.SwitchActor`))))
        (set `local.CanSwing-By` `Swing-By` :!label _label)
        (bind _asthird_person_character (cast `` Actor))
        (bind (_output_get _output_get_2) (set `self.Player` null _asthird_person_character))
        (`self.Set/Get_CanSwing-By` _output_get_2 (`self.CanSwingBy`) true)
        (set `/Game/Import/Blueprints/New_Hiraishin.ETOJammered` EtoJammaered (`.Player` (`self.Player`)))
        (bind _output_get_3 (set `/Game/Import/Blueprints/New_Hiraishin.JammingSpot` (`SceneComponent.K2_GetComponentLocation` (`self.ParticleZone`)) _player_2))
        (bind _output_get_4 (set `self.JammingSpot` _output_get_3))
        (set `/Game/Import/Blueprints/New_Hiraishin.ETOPosition` (- _returnvalue _output_get_4) _player_4)
        (if (`/Game/Import/Blueprints/New_Hiraishin.PlayETO` _player_4)
          (`self.K2_SetActorRotation` (`.Player` (`self.Player`)) (`KismetMathLibrary.FindLookAtRotation` (`SceneComponent.K2_GetComponentLocation` (`Actor.RootComponent` _player_4)) (`self.JammingSpot`)) false) ; エクレアを避雷針の中心に向けさせる
        )
        (set `/Game/Import/Blueprints/New_Hiraishin.HiraishinAxis` (`KismetMathLibrary.GreaterGreater_VectorRotator` (`KismetMathLibrary.MakeVector` _returnvalue_x _returnvalue_y) (struct :`Yaw` 90.0)) (`.Player` (`self.Player`)))
        (`self.SetJammeredEtoPosition` (`.Player` (`self.Player`)) (`self.JammingSpot`))))
    (:`Is Not Valid`
      (goto _label))))

(fn `UserConstructionScript`)