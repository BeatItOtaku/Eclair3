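; Naraku2_Blueprint is a pit-style hazard that sends the ThirdPersonCharacter back to a checkpoint on overlap.
; It hides the mesh and disables input, waits briefly, then teleports the player and restores both.
; GetLatestRespawnPoint picks the destination from all RespawnPoint_Blueprint actors by the latest CheckedTime among those marked Checked.
; A GetNearestActor distance helper is also defined but unused here.
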(event `self.ReceiveActorBeginOverlap`
  (params (OtherActor :type "Actor Object Reference"))
  (bind _player (`self.Player`))
  (bind _asthird_person_character (cast `/Game/ThirdPersonBP/Blueprints/ThirdPersonCharacter` OtherActor))
  (bind _output_get (set `self.Player` _asthird_person_character))
  (`SceneComponent.SetVisibility` (`Character.Mesh` _output_get) false false)
  (`self.DisableInput` _player null)
  (`KismetSystemLibrary.Delay` 0.1)
  (`|ExecutionSequence`
    (:`then_0`
      (bind _outactors (`GameplayStatics.GetAllActorsOfClass` "/Game/Blueprints/RespawnPoint_Blueprint.RespawnPoint_Blueprint_C"))
      (bind _latest (`self.Get Latest RespawnPoint` _outactors)))
    (:`then_1`
      (`self.K2_SetActorTransform` _player (`self.GetTransform` _latest) false false)
      (`SceneComponent.SetVisibility` (`Character.Mesh` (`self.Player`)) true false)
      (`self.EnableInput` (`self.Player`) null))))

(fn `Get Latest RespawnPoint`
  (params (SpawnPoints :type "Array of /Game/Blueprints/RespawnPoint_Blueprint Object Reference"))
  (returns (Latest :type "/Game/Blueprints/RespawnPoint_Blueprint Object Reference"))
  (locals (mLatest :type "/Game/Blueprints/RespawnPoint_Blueprint Object Reference") (mLatestTime :type "Float (double-precision)"))
  (for _array_element SpawnPoints
    (if (`/Game/Blueprints/RespawnPoint_Blueprint.Checked` _array_element)
      (bind _checkedtime (`/Game/Blueprints/RespawnPoint_Blueprint.CheckedTime` _array_element))
      (if (> _checkedtime (`local.mLatestTime`))
        (set `local.mLatest` _array_element)
        (set `local.mLatestTime` _checkedtime))))
  (return (`local.mLatest`)))

(fn `Get Nearest Actor`
  (params (Actors :type "Array of /Game/Blueprints/RespawnPoint_Blueprint Object Reference") (Player :type "Actor Object Reference"))
  (returns (Nearest :type "Actor Object Reference"))
  (locals (nearestactor :type "Actor Object Reference") (nearestdist :type "Float (double-precision)" :default 50000.0))
  (set `local.nearestactor` (`|GetArrayItem` Actors))
  (for _array_element Actors
    (bind _returnvalue (`KismetMathLibrary.VSize` (- (`self.K2_GetActorLocation` _array_element) (`self.K2_GetActorLocation` Player))))
    (if (> (`local.nearestdist`) _returnvalue)
      (set `local.nearestactor` _array_element)
      (set `local.nearestdist` _returnvalue)))
  (return (`local.nearestactor`)))

(fn `UserConstructionScript`)