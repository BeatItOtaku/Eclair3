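; SplineRail is a Blueprint that wraps a spline as a rail path, exposing distance-based queries.
; GetCurrentLocation converts a travelled distance to a world position, optionally wrapping it by modulo of spline length for looping.
; GetLength returns the spline length, and IsArrived reports whether a distance is within one unit of the end or beyond.
; Tick evaluates IsArrived but takes no action on the result.
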(event `self.ReceiveTick`
  (params (DeltaSeconds :type "Float (single-precision)"))
  (bind _isarrived (`self.IsArrived` (`self.Length`)))
  (if _isarrived
    _))

(fn `GetCurrentLocation`
  (params (Length :type "Float (double-precision)") (Loop :type Boolean))
  (returns (NewParam :type "Vector Structure"))
  (if Loop
    (set `self.Length` (mod Length (`SplineComponent.GetSplineLength` (`self.Spline`))))
    (else
      (set `self.Length` Length)))
  (return (`SplineComponent.GetLocationAtDistanceAlongSpline` (`self.Spline`) (`self.Length`) "World")))

(fn `GetLength`
  (returns (Length :type "Float (double-precision)"))
  (return (`SplineComponent.GetSplineLength` (`self.Spline`))))

(fn `IsArrived`
  (params (Length :type "Float (double-precision)"))
  (returns (IsArrived :type Boolean))
  (return (>= Length (- (`SplineComponent.GetSplineLength` (`self.Spline`)) 1.0))))

(fn `UserConstructionScript`)