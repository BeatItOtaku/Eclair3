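; Door actor with a skeletal mesh that can be opened by a set of linked switches.
; BeginPlay caches the mesh's door animation Blueprint instance.
; When UseSwitch is set, Tick loops over the switches, multiplying a ±1 flag and breaking at the first one off.
; IsOpen is therefore true only while every switch is on, or when none are linked.
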(event `self.ReceiveBeginPlay`
  (bind _asdoor_anim_blueprint (cast `/Game/Import/Blueprints/door_anim_Blueprint` (`SkeletalMeshComponent.GetAnimInstance` (`self.SkeletalMeshComponent`))))
  (set `self.DoorAnimBP` _asdoor_anim_blueprint))

(event `self.ReceiveTick`
  (params (DeltaSeconds :type "Float (single-precision)"))
  (if (`self.UseSwitch`)
    (set `self.SwitchOnCount` 1)
    (for _array_element _
      (bind _output_get (set `self.SwitchOnCount` (* (`self.SwitchOnCount`) (`KismetMathLibrary.SelectInt` 1 -1 (`/Game/Import/Blueprints/SwitchActor_Blueprint.SwitchOn` _array_element)))))
      (if (not (> _output_get 0))
        (break)))
    (set `self.IsOpen` (> (`self.SwitchOnCount`) 0))))

(fn `UserConstructionScript`)