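; A gimmick switch actor that the Eclair character can operate, showing its on/off state with blue and red lights.
; Overlapping its resizable box collider enables switching and spawns a use-prompt widget above the mesh; leaving removes both.
; Combined setter/getter functions expose the state; setting it fires on/off calls, updates lights, clears the prompt and optionally disables player input.
; The press-count setter only prints and stores, as its threshold-to-switch logic is disconnected.
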(event `self.ReceiveBeginPlay`
  (bind _redlight (`self.RedLight`))
  (bind _bluelight (`self.BlueLight`))
  (set `self.CurrentTime` (`self.LimitedTime`))
  (if (`self.SwitchOn`)
    (`SceneComponent.SetVisibility` _bluelight true true)
    (`SceneComponent.SetVisibility` _redlight false true)
    (else
      (`SceneComponent.SetVisibility` _bluelight false true)
      (`SceneComponent.SetVisibility` _redlight true true))))

(event `self.ReceiveTick`
  (params (DeltaSeconds :type "Float (single-precision)")))

(event `self.Collider.OnComponentBeginOverlap`
  (params (OverlappedComponent :type "PrimitiveComponent Object Reference") (OtherActor :type "Actor Object Reference") (OtherComp :type "PrimitiveComponent Object Reference") (OtherBodyIndex :type Integer) (bFromSweep :type Boolean) (SweepResult :type "HitResult Structure (by ref)"))
  (bind _aseclair_bp (cast `/Game/Import/ThirdPersonBP/Blueprints/EclairBP` OtherActor))
  (set `self.Eclair` _aseclair_bp)
  (bind _returnvalue (`|CreateWidget` "/Game/Base/Widget/ToolTip/UseGimmickUI.UseGimmickUI_C" null (+ (`SceneComponent.K2_GetComponentLocation` (`self.StaticMeshComponent`)) (0.0 0.0 250.0))))
  (bind _output_get (set `self.GimmickUI` _returnvalue))
  (`UserWidget.AddToViewport` _output_get 0)
  (`self.Set/Get CanSwitching` true true))

(event `self.Collider.OnComponentEndOverlap`
  (params (OverlappedComponent :type "PrimitiveComponent Object Reference") (OtherActor :type "Actor Object Reference") (OtherComp :type "PrimitiveComponent Object Reference") (OtherBodyIndex :type Integer))
  (cast `/Game/Import/ThirdPersonBP/Blueprints/EclairBP` OtherActor)
  (`/Game/Base/Widget/ToolTip/UseGimmickUI.Destroy` (`self.GimmickUI`))
  (`self.Set/Get CanSwitching` false true))

(fn `Set/Get CanSwitching`
  (params (`Input Value` :type Boolean) (IsSetter :type Boolean))
  (returns (`Output Value` :type Boolean))
  (if IsSetter
    (set `self.CanSwitching` `Input Value`)
    (else
      (return (`self.CanSwitching`)))))

(fn `Set/Get Switch On`
  (params (Input_SwitchOn :type Boolean) (IsSetter :type Boolean))
  (returns (output_SwitchOn :type Boolean))
  (bind _redlight (`self.RedLight`))
  (bind _bluelight (`self.BlueLight`))
  (if IsSetter
    (bind _output_get (set `self.SwitchOn` Input_SwitchOn))
    (if _output_get
      (`self.On Switch On`)
      (`SceneComponent.SetVisibility` _bluelight true true)
      (`SceneComponent.SetVisibility` _redlight false true)
      (else
        (`self.On Switch Off`)
        (`SceneComponent.SetVisibility` _bluelight false true)
        (`SceneComponent.SetVisibility` _redlight true true)))
    (`/Game/Base/Widget/ToolTip/UseGimmickUI.Destroy` (`self.GimmickUI`))
    (if (`self.PlayerUnmovable`)
      (`self.DisableInput` (`self.Eclair`) null))
    (else
      (return (`self.SwitchOn`)))))

(fn `SetRendaCount`
  (params (rendacount :type Integer))
  (locals (LimitRendaCount :type Integer :default 30))
  (`KismetSystemLibrary.PrintString` (`KismetStringLibrary.Conv_IntToString` rendacount))
  (bind _output_get (set `self.RendaCount` rendacount)))

(fn `UserConstructionScript`
  (`BoxComponent.SetBoxExtent` (`self.Collider`) (`self.BoxColliderScale`) true))