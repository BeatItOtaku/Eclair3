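; AkStateVolume is a volume actor that sets a Wwise State based on where the player character is, much like a prioritized post-process volume.
; It re-evaluates on any overlap begin or end, and at BeginPlay when Unbound.
; Each update scans all AkStateVolumes in the same StateGroup and applies the State of the highest-Priority one that is Unbound or overlaps the player.
; With no match, no fallback State is defined.
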(event `self.ReceiveBeginPlay`
  (if (`self.Unbound`)
    (`self.UpdateState` :!label _label)))

(event `self.ReceiveActorBeginOverlap`
  (params (OtherActor :type "Actor Object Reference"))
  (goto _label))

(event `self.CollisionComponent.OnComponentEndOverlap`
  (params (OverlappedComponent :type "PrimitiveComponent Object Reference") (OtherActor :type "Actor Object Reference") (OtherComp :type "PrimitiveComponent Object Reference") (OtherBodyIndex :type Integer))
  (goto _label))

(event `UpdateState`
  (bind _maxpriorityobject (`self.MaxPriorityObject`))
  (`|ExecutionSequence`
    (:`then_0`
      (set `self.MaxPriority` -1)
      (set `self.MaxPriorityObject` null))
    (:`then_1`
      (bind _outactors (`GameplayStatics.GetAllActorsOfClass` "AkStateVolume_C"))
      (for _array_element _outactors
        ;[1 1 1] 同一StateGroup判定
        (if (`KismetStringLibrary.EqualEqual_StrStr` (`self.StateGroup`) (`/Game/Sound/Blueprint/AkStateVolume.StateGroup` _array_element))
          ;[1 1 1] コリジョン判定
          (if (or (`/Game/Sound/Blueprint/AkStateVolume.Unbound` _array_element) (`PrimitiveComponent.IsOverlappingActor` (`TriggerBase.CollisionComponent` _array_element) (`GameplayStatics.GetPlayerCharacter` 0)))
            (bind _priority (`/Game/Sound/Blueprint/AkStateVolume.Priority` _array_element))
            ;[1 1 1] 優先度比較
            (if (> _priority (`self.MaxPriority`))
              (set `self.MaxPriority` _priority)
              (set `self.MaxPriorityObject` _array_element)))))
      (`AkGameplayStatics.SetState` (`KismetStringLibrary.Conv_StringToName` (`/Game/Sound/Blueprint/AkStateVolume.StateGroup` _maxpriorityobject)) (`KismetStringLibrary.Conv_StringToName` (`/Game/Sound/Blueprint/AkStateVolume.State` _maxpriorityobject))))))

(fn `UserConstructionScript`)