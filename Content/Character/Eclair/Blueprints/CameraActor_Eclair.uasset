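; Standalone follow camera actor for the Eclair character that becomes the player's view target and supports enemy lock-on.
; Each tick it sits 100 units above the player pawn, copying control rotation or, when locked, facing NearestEnemy.
; OnLockOn toggles the lock and picks a target by minimum distance among "Enemy"-tagged actors within a 60-degree view cone.
; That minimum's index is applied to the unfiltered enemy list, so the chosen target can differ.
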(event `self.ReceiveBeginPlay`
  (`PlayerController.SetViewTargetWithBlend` (`GameplayStatics.GetPlayerController` 0) self 0.0 "VTBlend_Linear" 0.0 false)
  (set `self.Pawn_Ealcir` (`GameplayStatics.GetPlayerPawn` 0)))

(event `self.ReceiveTick`
  (params (DeltaSeconds :type "Float (single-precision)"))
  (`self.K2_SetActorLocation` (`self.SetCameraLocation`))
  (`self.K2_SetActorRotation` (`self.SetCameraRotation`)))

(event `OnLockOn`
  (set `self.IsLockOn` (not (`self.IsLockOn`)))
  (`KismetArrayLibrary.Array_Clear` (`self.Ecemies`))
  (`KismetArrayLibrary.Array_Clear` (`self.DistanceOfEnemies`))
  (bind _outactors (`GameplayStatics.GetAllActorsWithTag` "Enemy"))
  (bind _output_get (set `self.Ecemies` _outactors))
  (for _array_element _output_get
    (if (`self.IsActorOnCamera` _array_element)
      (`KismetArrayLibrary.Array_Add` (`self.DistanceOfEnemies`) (`KismetMathLibrary.VSize` (- (`SceneComponent.K2_GetComponentLocation` (`Actor.RootComponent` _array_element)) (`SceneComponent.K2_GetComponentLocation` (`self.FollowCamera`)))))))
  (bind _output_get_2 (set `self.NearestEnemy` (`|GetArrayItem` (`self.Ecemies`) (`KismetMathLibrary.MinOfFloatArray` (`self.DistanceOfEnemies`)))))
  (`KismetSystemLibrary.PrintString` (`KismetSystemLibrary.GetDisplayName` _output_get_2)))

(fn `GetLookAtRotator`
  (params (Actor :type "Actor Object Reference"))
  (returns (LookAtRotator :type "Rotator Structure"))
  (return (`KismetMathLibrary.FindLookAtRotation` (`SceneComponent.K2_GetComponentLocation` (`self.FollowCamera`)) (`self.K2_GetActorLocation` Actor))))

(fn `IsActorOnCamera`
  (params (Actor :type "Actor Object Reference"))
  (returns (isActorOnCamera :type Boolean))
  (return (< (`KismetMathLibrary.DegAcos` (`KismetMathLibrary.Dot_VectorVector` (`SceneComponent.GetForwardVector` (`self.FollowCamera`)) (`KismetMathLibrary.GetForwardVector` (`self.GetLookAtRotator` Actor)))) 60.0)))

(fn `SetCameraLocation`
  (returns (CameraLocation :type "Vector Structure"))
  (bind (_returnvalue_x _returnvalue_y _returnvalue_z) (`KismetMathLibrary.BreakVector` (`self.K2_GetActorLocation` (`self.Pawn_Ealcir`))))
  (return (`KismetMathLibrary.MakeVector` _returnvalue_x _returnvalue_y (+ _returnvalue_z 100.0))))

(fn `SetCameraRotation`
  (returns (ReturnValue :type "Rotator Structure"))
  (locals (ReturnRotateValue :type "Rotator Structure"))
  (if (`self.IsLockOn`)
    (set `local.ReturnRotateValue` (`self.GetLookAtRotator` (`self.NearestEnemy`)))
    (else
      (set `local.ReturnRotateValue` (`Pawn.GetControlRotation` (`self.Pawn_Ealcir`)))))
  (return (`local.ReturnRotateValue`)))

(fn `UserConstructionScript`)